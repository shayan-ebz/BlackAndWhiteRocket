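; BP_Bomb is a bomb objective that the Paper Captain defuses by touching it.
; When its Sphere overlaps a BP_PaperCaptain, it sets DefusedBomb on the player pawn and destroys itself.
; It then shows the WBP_BackToRocket widget, plays the task-complete sound and pauses the game.
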(event OnComponentBeginOverlap(Sphere)
  (params (OverlappedComponent :type Primitive%20Component%20Object%20Reference) (OtherActor :type Actor%20Object%20Reference) (OtherComp :type Primitive%20Component%20Object%20Reference) (OtherBodyIndex :type Integer) (bFromSweep :type Boolean) (SweepResult :type Hit%20Result%20Structure%20%28by%20ref%29))
  (if (== (Utilities|GetClass OtherActor) "/Game/_Blueprint/GameLogics/BP_PaperCaptain.BP_PaperCaptain_C")
    (bind _asbp_paper_captain (Utilities|Casting|CastToBP_PaperCaptain (Game|Player|GetPlayerPawn 0)))
    (Variables|/Game/_Blueprint/GameLogics/BP_PaperCaptain.BP_PaperCaptain_C|SetbDefusedBomb _asbp_paper_captain true)
    (Actor|DestroyActor)
    (bind _returnvalue (UserInterface|CreateWidget "/Game/_Blueprint/HUD/Menu/WBP_BackToRocket.WBP_BackToRocket_C"))
    (UserInterface|Viewport|AddtoViewport _returnvalue 0)
    (Audio|PlaySound2D "/Game/ImportedContent/Sounds/task_complete_Cue.task_complete_Cue" 1.0 1.0 0.0 0 0)
    (Game|SetGamePaused true)))

(event EventBeginPlay)

(event Collision|EventActorBeginOverlap
  (params (OtherActor :type Actor%20Object%20Reference)))

(event EventTick
  (params (DeltaSeconds :type Float%20%28single-precision%29)))

(fn ConstructionScript)