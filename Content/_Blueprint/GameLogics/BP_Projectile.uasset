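; Projectile actor that destroys itself when its sphere begins overlapping anything and kills the actor it overlaps if that is exactly a BP_AIEnemy.
; The kill runs once, directly from the projectile: it toggles the enemy's Die and Sprite visibility, stops its movement and disables capsule collision.
; It then gives the enemy a short life span for delayed removal and plays a death sound, alongside a debug print.
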(event OnComponentHit(Sphere)
  (params (HitComponent :type Primitive%20Component%20Object%20Reference) (OtherActor :type Actor%20Object%20Reference) (OtherComp :type Primitive%20Component%20Object%20Reference) (NormalImpulse :type Vector :default "0, 0, 0") (Hit :type Hit%20Result%20Structure%20%28by%20ref%29)))

(event OnComponentBeginOverlap(Sphere)
  (params (OverlappedComponent :type Primitive%20Component%20Object%20Reference) (OtherActor :type Actor%20Object%20Reference) (OtherComp :type Primitive%20Component%20Object%20Reference) (OtherBodyIndex :type Integer) (bFromSweep :type Boolean) (SweepResult :type Hit%20Result%20Structure%20%28by%20ref%29))
  (Actor|DestroyActor)
  ;[1 1 1] AI Die
  (if (== (Utilities|GetClass OtherActor) "/Game/_Blueprint/GameLogics/BP_AIEnemy.BP_AIEnemy_C")
    (Development|PrintString "Ai Died")
    (bind _asbp_aienemy (Utilities|Casting|CastToBP_AIEnemy OtherActor))
    (Utilities|FlowControl|DoOnce false
      (:Completed
        (Rendering|ToggleVisibility (Variables|/Game/_Blueprint/GameLogics/BP_AIEnemy.BP_AIEnemy_C|GetDie _asbp_aienemy) false)
        (Rendering|ToggleVisibility (Variables|/Script/Paper2D.PaperCharacter|GetSprite _asbp_aienemy) false)
        (Components|Activation|Deactivate (Variables|/Script/Engine.Character|GetCharacterMovement _asbp_aienemy))
        (Collision|SetCollisionEnabled (Variables|/Script/Engine.Character|GetCapsuleComponent _asbp_aienemy) "NoCollision")
        (Actor|SetLifeSpan _asbp_aienemy 0.8)
        (Audio|PlaySound2D "/Game/ImportedContent/Sounds/hdeath2_Cue.hdeath2_Cue" 1.0 1.0 0.0 0 0)))))

(event EventBeginPlay)

(event Collision|EventActorBeginOverlap
  (params (OtherActor :type Actor%20Object%20Reference)))

(event EventTick
  (params (DeltaSeconds :type Float%20%28single-precision%29)))

(fn ConstructionScript)