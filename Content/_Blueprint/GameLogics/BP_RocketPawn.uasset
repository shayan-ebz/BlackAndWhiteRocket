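; Paper2D rocket pawn that explodes and restarts the level on a crash or hard landing.
; HitDetector hits trigger destruction once, while PaperRocket hits do so only when vertical speed reaches a threshold.
; Destruction plays a boom sound, swaps idle and power-up flipbooks for the destroy one, then restarts via a delayed console command.
; OpenNextLevel picks the next map from the current level name but is not called in this graph.
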(event OnComponentHit(HitDetector)
  (params (HitComponent :type Primitive%20Component%20Object%20Reference) (OtherActor :type Actor%20Object%20Reference) (OtherComp :type Primitive%20Component%20Object%20Reference) (NormalImpulse :type Vector :default "0, 0, 0") (Hit :type Hit%20Result%20Structure%20%28by%20ref%29))
  (bind _powerup_fb (Variables|Default|GetPowerUp_FB))
  (bind _idle_fb (Variables|Default|GetIdle_FB))
  ;[0 0.7791 1] play rocket destory animation then restart the level
  (Utilities|FlowControl|DoOnce false
    (:Completed
      (Utilities|FlowControl|Sequence
        (:then_0
          (Audio|PlaySound2D "/Game/ImportedContent/Sounds/RocketBoom_Cue.RocketBoom_Cue" 1.0 1.0 0.0 0 0)
          (Rendering|ToggleVisibility (Variables|Default|GetDestroy_FB) false)
          (if (Rendering|IsVisible _idle_fb)
            (Rendering|ToggleVisibility _idle_fb false))
          (if (Rendering|IsVisible _powerup_fb)
            (Rendering|ToggleVisibility _powerup_fb false)))
        (:then_1
          (Audio|PlaySound2D "/Game/ImportedContent/Sounds/RocketBoom_Cue.RocketBoom_Cue" 1.0 1.0 0.0 0 0)
          (Utilities|FlowControl|Delay 0.5)
          (Development|ExecuteConsoleCommand (Game|GetPlayerController 0) "RestartLevel" 0))))))

(event OnComponentHit(PaperRocket)
  (params (HitComponent :type Primitive%20Component%20Object%20Reference) (OtherActor :type Actor%20Object%20Reference) (OtherComp :type Primitive%20Component%20Object%20Reference) (NormalImpulse :type Vector :default "0, 0, 0") (Hit :type Hit%20Result%20Structure%20%28by%20ref%29))
  (bind _destroy_fb (Variables|Default|GetDestroy_FB))
  (bind _idle_fb (Variables|Default|GetIdle_FB))
  (bind _powerup_fb (Variables|Default|GetPowerUp_FB))
  (bind _paperrocket (Variables|Default|GetPaperRocket))
  (bind _returnvalue (Transformation|GetComponentVelocity _paperrocket))
  (bind _z (Math|Vector|BreakVector _returnvalue))
  ;[0 0.8504 1] Landing Velocity Condition
  (Development|PrintString "Hello" true true "(R=0.000000,G=0.660000,B=1.000000,A=1.000000)" _z)
  (if (>= (Math|Float|Absolute(Float) _z) 2e+02)
    (Audio|PlaySound2D "/Game/ImportedContent/Sounds/RocketBoom_Cue.RocketBoom_Cue" 1.0 1.0 0.0 0 0)
    (Utilities|FlowControl|Sequence
      (:then_0
        (if (not (Rendering|IsVisible _destroy_fb))
          (Rendering|ToggleVisibility _destroy_fb false)
          (if (Rendering|IsVisible _idle_fb)
            (Rendering|ToggleVisibility _idle_fb false))
          (if (Rendering|IsVisible _powerup_fb)
            (Rendering|ToggleVisibility _powerup_fb false))))
      (:then_1
        (Utilities|FlowControl|Delay 1.0)
        (Development|ExecuteConsoleCommand (Game|GetPlayerController 0) "RestartLevel" 0)))))

(event EventBeginPlay)

(event Collision|EventActorBeginOverlap
  (params (OtherActor :type Actor%20Object%20Reference)))

(event EventTick
  (params (DeltaSeconds :type Float%20%28single-precision%29)))

(fn ConstructionScript)

(fn OpenNextLevel
  (bind _returnvalue (Game|GetCurrentLevelName true))
  (if (Utilities|Enum|Equal(Enum) _returnvalue "map1_0")
    (Game|OpenLevel(byName) "map1_1")
    (else
      (Game|OpenLevel(byName) "map2_1"))))